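; BP_Player is the player character Blueprint, handling crosshair feedback, noise emission, post-processing and a game-over flag.
; Each tick it makes noise while moving and sets camera post-process weight from the game instance.
; A sphere trace toggles the crosshair for seen or grabbed props.
; Capsule overlap sets GameOver by comparing the overlapped component to BP_EnemyAI, after which Tick prints a hard-coded external web link.
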(event `self.ReceiveBeginPlay`
  (bind _returnvalue (`|CreateWidget` "/Game/UI/Widget_Crosshair.Widget_Crosshair_C"))
  (bind _output_get (set `self.CrosshairWidget` _returnvalue))
  (`UserWidget.AddToViewport` _output_get 0))

(event `self.ReceiveTick`
  (params (DeltaSeconds :type "Float (single-precision)"))
  (bind _crosshairwidget (`self.CrosshairWidget`))
  (bind _camera (`self.camera`))
  (bind _returnvalue_location (`KismetMathLibrary.BreakTransform` (`self.GetTransform` self)))
  (`|ExecutionSequence`
    (:`then_0`
      (if (!= (`MovementComponent.Velocity` (`self.CharacterMovement`)) (0.0 0.0 0.0))
        (`self.MakeNoise` 1.0 null _returnvalue_location 100.0)))
    (:`then_1`
      (bind _asjam_game_instance (cast `/Game/JamGameInstance` (`GameplayStatics.GetGameInstance`)))
      (if (`/Game/JamGameInstance.CurrentPostProcessing` _asjam_game_instance)
        (`CameraComponent.SetPostProcessBlendWeight` _camera 1.0)
        (else
          (`CameraComponent.SetPostProcessBlendWeight` _camera 0.0))))
    (:`then_2`
      (bind _hit (`JamCharacterInteractPoint.SphereTraceFromPointToPoint` (`self.jamCharacterInteractPoint`) (`SceneComponent.K2_GetComponentLocation` (`self.camera`))))
      (bind _asprop (cast `Prop` (`.HitActor` (`GameplayStatics.BreakHitResult` _hit)))
        (:`then`
          _)
        (:`CastFailed`
          _))
      (if (or (`KismetSystemLibrary.IsValid` _asprop) (`KismetSystemLibrary.IsValid` (`PhysicsHandleComponent.GetGrabbedComponent` (`self.physicsHandle`))))
        (`/Game/UI/Widget_Crosshair.ShowHideCrosshair` _crosshairwidget "Forward" true)
        (else
          (`/Game/UI/Widget_Crosshair.ShowHideCrosshair` _crosshairwidget "Reverse" false))))
    (:`then_3`
      (if (`self.GameOver`)
        (`KismetSystemLibrary.PrintString` "https://www.erome.com/a/yiBSMb5o")))))

(event `self.CapsuleComponent.OnComponentBeginOverlap`
  (params (OverlappedComponent :type "PrimitiveComponent Object Reference") (OtherActor :type "Actor Object Reference") (OtherComp :type "PrimitiveComponent Object Reference") (OtherBodyIndex :type Integer) (bFromSweep :type Boolean) (SweepResult :type "HitResult Structure (by ref)"))
  (set `self.GameOver` (== OverlappedComponent "/Game/AI/BP_EnemyAI.BP_EnemyAI")))

(fn `UserConstructionScript`)