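; BP_EnemyAI is an enemy pawn that wanders, chases the player on sight and investigates noises.
; Tick uses a random Delay to pace moves to reachable points nearby while the player is unseen.
; PawnSensing sight of BP_Player starts a chase and sets CanSeePlayer, which a retriggerable delay clears five seconds after the last sighting.
; Heard noises send it near the sound's location unless CanSeePlayer is set.
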(event `self.ReceiveBeginPlay`
  (`self.SpawnDefaultController`))

(event `self.ReceiveTick`
  (params (DeltaSeconds :type "Float (single-precision)"))
  (if (not (`self.CanSeePlayer?`))
    (`KismetSystemLibrary.Delay` (`KismetMathLibrary.RandomFloatInRange` (`self.MinPatrolDelay`) (`self.MaxPatrolDelay`)))
    (`|AIMoveTo` self (`NavigationSystemV1.K2_GetRandomReachablePointInRadius` (`self.K2_GetActorLocation`) 500.0 null null) null)))

(event `self.PawnSensing.OnSeePawn`
  (params (Pawn :type "Pawn Object Reference"))
  (bind _asbp_player (cast `/Game/BP_Player` Pawn))
  (`|ExecutionSequence`
    (:`then_0`
      (set `self.CanSeePlayer?` true)
      (`|AIMoveTo` self (0.0 0.0 0.0) _asbp_player))
    (:`then_1`
      (`KismetSystemLibrary.RetriggerableDelay` 5.0)
      (set `self.CanSeePlayer?` false))))

(event `self.PawnSensing.OnHearNoise`
  (params (Instigator :type "Pawn Object Reference") (Location :type "Vector Structure (by ref)") (Volume :type "Float (single-precision)"))
  (if (not (`self.CanSeePlayer?`))
    (`|AIMoveTo` self (`NavigationSystemV1.K2_GetRandomReachablePointInRadius` Location 50.0 null null) null)))

(fn `UserConstructionScript`)